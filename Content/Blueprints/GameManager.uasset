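; GameManager is a Blueprint that opens a door once enough Leaver actors in the level have been swapped.
; On BeginPlay it finds every Leaver, binds its swap event to a counter, and stores the total as the required count.
; Each swap event increments the counter, and when it equals that total the manager broadcasts the open-door dispatcher.
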(event `self.ReceiveBeginPlay`
  (bind _outactors (`GameplayStatics.GetAllActorsOfClass` "/Game/Blueprints/Leaver.Leaver_C"))
  (for _array_element _outactors
    (add `/Game/Blueprints/Leaver.Leaver swapped` _array_element (delegate `Add Swapped Leaver`)))
  (set `self.needed leavers` (`KismetArrayLibrary.Array_Length` _outactors)))

(event `Add Swapped Leaver`
  (bind _leavers (`self.leavers`))
  (`/Engine/EditorBlueprintResources/StandardMacros.IncrementInt` _leavers
    (:`  `
      (if (== _leavers (`self.needed leavers`))
        (`self.callOnOpenDoor`)))))

(fn `UserConstructionScript`)