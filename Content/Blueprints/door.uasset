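; Door actor that opens and closes in response to events from other level actors.
; On BeginPlay it finds the GameManager and MassBlockCounter, binding to their open and close dispatchers respectively.
; Opening instantly drops the static mesh along Z, while closing raises it by the same offset, each with a 2D sound.
; Closing is guarded by a DoOnce, so it runs only once, whereas opening has no guard.
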(event `self.ReceiveBeginPlay`
  (bind _returnvalue (`GameplayStatics.GetActorOfClass` "/Game/Blueprints/GameManager.GameManager_C"))
  (add `/Game/Blueprints/GameManager.callOnOpenDoor` _returnvalue (delegate `opendoor`))
  (bind _returnvalue_2 (`GameplayStatics.GetActorOfClass` "/Game/Blueprints/MassBlockCounter.MassBlockCounter_C"))
  (add `/Game/Blueprints/MassBlockCounter.closeDoor` _returnvalue_2 (delegate `closedoor`)))

(event `opendoor`
  (`SceneComponent.K2_AddRelativeLocation` (`self.StaticMesh`) (0.0 0.0 -2000.0) false false)
  (`GameplayStatics.PlaySound2D` "/Game/sounds/sfx/drzwi.drzwi" 1.0 1.0 0.0 null null))

(event `closedoor`
  (`/Engine/EditorBlueprintResources/StandardMacros.DoOnce` false
    (:`Completed`
      (`SceneComponent.K2_AddRelativeLocation` (`self.StaticMesh`) (0.0 0.0 2000.0) false false)
      (`GameplayStatics.PlaySound2D` "/Game/sounds/sfx/drzwi_zamykanie.drzwi_zamykanie" 1.0 1.0 0.0 null null))))

(fn `UserConstructionScript`)