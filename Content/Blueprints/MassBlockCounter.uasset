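; MassBlockCounter is a pressure slab that triggers a door-closing call once it has been left empty for a countdown.
; It starts pressed; box overlaps lower it for a MassBlock with positive mass and raise it when a MassBlock or WazaZGwiazda leaves, playing sounds.
; Tick resets the timer while occupied, otherwise counts down and calls CloseDoor every frame after expiry, printing the time for debugging.
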(event `self.ReceiveBeginPlay`
  (set `self.someting is on slab` true)
  (`SceneComponent.K2_AddRelativeLocation` (`self.spod`) (0.0 0.0 -10.0) false false)
  (set `self.time` 5.0))

(event `self.Box.OnComponentBeginOverlap`
  (params (OverlappedComponent :type "PrimitiveComponent Object Reference") (OtherActor :type "Actor Object Reference") (OtherComp :type "PrimitiveComponent Object Reference") (OtherBodyIndex :type Integer) (bFromSweep :type Boolean) (SweepResult :type "HitResult Structure (by ref)"))
  (bind _asmass_block (cast `/Game/Blueprints/MassBlock` OtherActor))
  (if (> (`/Game/Blueprints/MassBlock.mass` _asmass_block) 0.0)
    (bind _output_get (set `self.someting is on slab` true))
    (if _output_get
      (`SceneComponent.K2_AddRelativeLocation` (`self.spod`) (0.0 0.0 -10.0) false false)
      (`GameplayStatics.PlaySound2D` "/Game/sounds/sfx/zejscie_z_plytki.zejscie_z_plytki" 1.0 1.0 0.0 null null))))

(event `self.Box.OnComponentEndOverlap`
  (params (OverlappedComponent :type "PrimitiveComponent Object Reference") (OtherActor :type "Actor Object Reference") (OtherComp :type "PrimitiveComponent Object Reference") (OtherBodyIndex :type Integer))
  (cast `/Game/Blueprints/MassBlock` OtherActor
    (:`then`
      _)
    (:`CastFailed`
      (cast `/Game/Blueprints/WazaZGwiazda` OtherActor)))
  (set `self.someting is on slab` false)
  (`SceneComponent.K2_AddRelativeLocation` (`self.spod`) (0.0 0.0 10.0) false false)
  (`GameplayStatics.PlaySound2D` "/Game/sounds/sfx/wchodzenie_na_plytke.wchodzenie_na_plytke" 1.0 1.0 0.0 null null))

(event `self.ReceiveTick`
  (params (DeltaSeconds :type "Float (single-precision)"))
  (`KismetSystemLibrary.PrintString` (`KismetStringLibrary.Conv_DoubleToString` (`self.time`)) true true (struct :`G` 0.66 :`B` 1.0 :`A` 1.0) 2.0 "1")
  (if (`self.someting is on slab`)
    (set `self.time` 5.0)
    (else
      (bind _output_get (set `self.time` (- (`self.time`) DeltaSeconds)))
      (if (<= _output_get 0.0)
        (`self.closeDoor`)))))

(fn `UserConstructionScript`)