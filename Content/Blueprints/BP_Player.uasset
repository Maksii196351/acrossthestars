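; Player Blueprint that runs the camera-flight teleport transitions between levels and can spawn the HUD or ending widget at start.
; Altar's world change or BP_Staruch's game end sends Camera1 flying out on Tick before opening Gra2 or LastLevel, with debug H triggering both.
; Without spawned widgets, an intro flight with light and sound returns to the main camera and enables input.
; Tick also sets the mesh by whether this is the player's pawn.
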(event Custom|CustomEvent
  (Components|Activation|SetActive (Variables|Default|GetCamera) false true)
  (Components|Activation|SetActive (Variables|Default|GetCamera1) true false)
  (Variables|Default|Setfly%20camera true)
  (Utilities|FlowControl|Delay 6.0)
  (Game|OpenLevel(byObjectReference) "/Game/LastLevel.LastLevel"))

(event Custom|change%20world
  (Components|Activation|SetActive (Variables|Default|GetCamera) false true)
  (Components|Activation|SetActive (Variables|Default|GetCamera1) true false)
  (Variables|Default|Setfly%20camera true)
  (Utilities|FlowControl|Delay 6.0)
  (Game|OpenLevel(byObjectReference) "/Game/Gra2.Gra2"))

(event EventBeginPlay
  (bind _create_hud_at_spawn (Variables|Default|Getcreate%20hud%20at%20spawn))
  (bind _create_ending_at_spawn (Variables|Default|Getcreate%20ending%20at%20spawn))
  (Utilities|FlowControl|Sequence
    (:then_0
      (bind _returnvalue (Actor|GetActorOfClass "/Game/Blueprints/altar.altar_C"))
      (EventDispatchers|BindEventtoChangeworld _returnvalue (delegate Custom|change%20world))
      (bind _returnvalue_2 (Actor|GetActorOfClass "/Game/gosc/BP_Staruch.BP_Staruch_C"))
      (EventDispatchers|BindEventtoGameEnd2 _returnvalue_2 (delegate Custom|CustomEvent)))
    (:then_1
      (Utilities|FlowControl|Delay 0.2)
      (if (and (not _create_ending_at_spawn) (not _create_hud_at_spawn))
        (Variables|Default|Setcameracome true)
        (Components|Activation|SetActive (Variables|Default|GetCamera) false true)
        (Components|Activation|SetActive (Variables|Default|GetCamera1) true false)))
    (:then_2
      (if _create_hud_at_spawn
        (bind _returnvalue_3 (Game|ConstructObjectfromClass "/Game/Blueprints/Hud.Hud_C"))
        (UserInterface|Viewport|AddtoViewport _returnvalue_3 0)))
    (:then_3
      (if _create_ending_at_spawn
        (bind _returnvalue_4 (Game|ConstructObjectfromClass "/Game/Blueprints/ending.ending_C"))
        (UserInterface|Viewport|AddtoViewport _returnvalue_4 0)))))

(event Collision|EventActorBeginOverlap
  (params (OtherActor :type Actor%20Object%20Reference)))

(event EventTick
  (params (DeltaSeconds :type Float%20%28single-precision%29))
  (Utilities|FlowControl|Sequence
    (:then_0
      (if (Variables|Default|Getfly%20camera)
        (Transformation|AddRelativeLocation (Variables|Default|GetCamera1) (Math|Vector|MakeVector (* DeltaSeconds -1e+03) 0.0 0.0) false false)
        (Utilities|FlowControl|DoOnce false
          (:Completed
            (Rendering|SetVisibility (Variables|Default|GetPointLight) true false)
            (Audio|PlaySound2D "/Game/sounds/sfx/teleport1.teleport1" 1.0 1.0 0.0 0 0)
            (Utilities|FlowControl|Delay 6.0)
            (Variables|Default|Setfly%20camera false)))))
    (:then_1
      (if (Variables|Default|Getcameracome)
        (Transformation|AddRelativeLocation (Variables|Default|GetCamera1) (Math|Vector|MakeVector (* DeltaSeconds 1e+03) 0.0 0.0) false false)
        (Utilities|FlowControl|DoOnce false
          (:Completed
            (Rendering|SetVisibility (Variables|Default|GetPointLight) true false)
            (Audio|PlaySound2D "/Game/sounds/sfx/teleport2.teleport2" 1.0 1.0 0.0 0 0)
            (Utilities|FlowControl|Delay 6.0)
            (Variables|Default|Setcameracome false)
            (Rendering|SetVisibility (Variables|Default|GetPointLight) true false)
            (Components|Activation|SetActive (Variables|Default|GetCamera1) false true)
            (Components|Activation|SetActive (Variables|Default|GetCamera) true false)
            (Input|EnableInput (Game|GetPlayerController 0))))))
    (:then_2
      (if (== self (Game|Player|GetPlayerPawn 0))
        (Components|SkeletalMesh|SetSkeletalMeshAsset (Variables|Character|GetMesh) 0)
        (else
          (Components|SkeletalMesh|SetSkeletalMeshAsset (Variables|Character|GetMesh) "/Game/gosc/chlop2.chlop2"))))))

(event EventPosses
  (Pawn|Possess (Game|GetPlayerController 0) self))

(event Input|KeyboardEvents|DebugKeyH
  (params (Key :type Key%20Structure :default "None") (ActionValue :type Input%20Action%20Value%20Structure))
  (:Pressed
    (Components|Activation|SetActive (Variables|Default|GetCamera) false true)
    (Components|Activation|SetActive (Variables|Default|GetCamera1) true false)
    (Variables|Default|Setfly%20camera true)
    (Utilities|FlowControl|Delay 6.0)
    (Game|OpenLevel(byObjectReference) "/Game/LastLevel.LastLevel")))

(event Input|KeyboardEvents|DebugKeyH
  (params (Key :type Key%20Structure :default "None") (ActionValue :type Input%20Action%20Value%20Structure))
  (:Pressed
    (Components|Activation|SetActive (Variables|Default|GetCamera) false true)
    (Components|Activation|SetActive (Variables|Default|GetCamera1) true false)
    (Variables|Default|Setfly%20camera true)
    (Utilities|FlowControl|Delay 6.0)
    (Game|OpenLevel(byObjectReference) "/Game/Gra2.Gra2")))

(fn ConstructionScript)