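; Pistons is a three-pad end-of-game trigger that opens the Ending level once all three boxes are occupied at the same time.
; Each box's overlap events set its flag for actors with "BP_Player" in their display name and fire GameEnd on entry.
; The flags are checked on GameEnd and every Tick, behind a DoOnce, with debug prints.
; BeginPlay also enables FlyCamera on the local player.
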(event `self.ReceiveBeginPlay`
  (add `self.game end` (delegate `CustomEvent_0`))
  (bind _outactors (`GameplayStatics.GetAllActorsOfClass` "/Game/Blueprints/BP_Player.BP_Player_C"))
  (for _array_element _outactors
    (bind _asbp_player (cast `/Game/Blueprints/BP_Player` _array_element))
    (if (== _asbp_player (`GameplayStatics.GetPlayerPawn` 0))
      (set `/Game/Blueprints/BP_Player.fly camera` true _asbp_player))))

(event `CustomEvent_0`
  (if (and (`self.1IsOn`) (`self.2IsOm`) (`self.3IsOn`)) :!label _label
    (`/Engine/EditorBlueprintResources/StandardMacros.DoOnce` false
      (:`Completed`
        (set `/Game/Blueprints/BP_Player.fly camera` true (stale `self.ReceiveBeginPlay` _array_element))
        (`GameplayStatics.OpenLevelBySoftObjectPtr` "/Game/ending.ending")))))

(event `self.ReceiveTick`
  (params (DeltaSeconds :type "Float (single-precision)"))
  (bind _1ison (`self.1IsOn`))
  (bind _2isom (`self.2IsOm`))
  (bind _3ison (`self.3IsOn`))
  (`|ExecutionSequence`
    (:`then_0`
      (goto _label))
    (:`then_1`
      (`KismetSystemLibrary.PrintString` (`KismetStringLibrary.Concat_StrStr` (`KismetStringLibrary.Conv_BoolToString` _1ison) (`KismetStringLibrary.Conv_BoolToString` _2isom) (`KismetStringLibrary.Conv_BoolToString` _3ison) (`KismetStringLibrary.Conv_BoolToString` (and _1ison _2isom _3ison))) true true (struct :`G` 0.66 :`B` 1.0 :`A` 1.0) 2.0 "ng"))))

(event `self.Box2.OnComponentBeginOverlap`
  (params (OverlappedComponent :type "PrimitiveComponent Object Reference") (OtherActor :type "Actor Object Reference") (OtherComp :type "PrimitiveComponent Object Reference") (OtherBodyIndex :type Integer) (bFromSweep :type Boolean) (SweepResult :type "HitResult Structure (by ref)"))
  (if (`KismetStringLibrary.Contains` (`KismetSystemLibrary.GetDisplayName` OtherActor) "BP_Player")
    (set `self.1IsOn` true)
    (`self.game end`)))

(event `self.Box2.OnComponentEndOverlap`
  (params (OverlappedComponent :type "PrimitiveComponent Object Reference") (OtherActor :type "Actor Object Reference") (OtherComp :type "PrimitiveComponent Object Reference") (OtherBodyIndex :type Integer))
  (if (`KismetStringLibrary.Contains` (`KismetSystemLibrary.GetDisplayName` OtherActor) "BP_Player")
    (set `self.1IsOn` false)))

(event `self.Box1.OnComponentBeginOverlap`
  (params (OverlappedComponent :type "PrimitiveComponent Object Reference") (OtherActor :type "Actor Object Reference") (OtherComp :type "PrimitiveComponent Object Reference") (OtherBodyIndex :type Integer) (bFromSweep :type Boolean) (SweepResult :type "HitResult Structure (by ref)"))
  (`KismetSystemLibrary.PrintString` "Hello")
  (if (`KismetStringLibrary.Contains` (`KismetSystemLibrary.GetDisplayName` OtherActor) "BP_Player")
    (set `self.2IsOm` true)
    (`self.game end`)))

(event `self.Box1.OnComponentEndOverlap`
  (params (OverlappedComponent :type "PrimitiveComponent Object Reference") (OtherActor :type "Actor Object Reference") (OtherComp :type "PrimitiveComponent Object Reference") (OtherBodyIndex :type Integer))
  (if (`KismetStringLibrary.Contains` (`KismetSystemLibrary.GetDisplayName` OtherActor) "BP_Player")
    (set `self.2IsOm` false)))

(event `self.Box.OnComponentBeginOverlap`
  (params (OverlappedComponent :type "PrimitiveComponent Object Reference") (OtherActor :type "Actor Object Reference") (OtherComp :type "PrimitiveComponent Object Reference") (OtherBodyIndex :type Integer) (bFromSweep :type Boolean) (SweepResult :type "HitResult Structure (by ref)"))
  (bind _returnvalue (`KismetStringLibrary.Contains` (`KismetSystemLibrary.GetDisplayName` OtherActor) "BP_Player"))
  (`KismetSystemLibrary.PrintString` (`KismetStringLibrary.Conv_BoolToString` _returnvalue))
  (if _returnvalue
    (set `self.3IsOn` true)
    (`self.game end`)))

(event `self.Box.OnComponentEndOverlap`
  (params (OverlappedComponent :type "PrimitiveComponent Object Reference") (OtherActor :type "Actor Object Reference") (OtherComp :type "PrimitiveComponent Object Reference") (OtherBodyIndex :type Integer))
  (if (`KismetStringLibrary.Contains` (`KismetSystemLibrary.GetDisplayName` OtherActor) "BP_Player")
    (set `self.3IsOn` false)))

(fn `UserConstructionScript`)