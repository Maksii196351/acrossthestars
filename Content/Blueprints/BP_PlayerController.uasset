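; Player controller for a body-swapping game: it drives movement and look for the possessed pawn, plus level restart and quit keys.
; BodySwap traces from the current BP_Player's camera and messages a hit BP_Player to take possession, then resets the trace ignore list.
; Interact uses a shorter trace to message the hit actor and grab its component by physics handle, with Tick pulling it to the GrabPoint.
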(event `self.ReceiveBeginPlay`
  (bind _outactors (`GameplayStatics.GetAllActorsOfClass` "/Game/Blueprints/BP_Player.BP_Player_C"))
  (for _array_element _outactors
    (set `self.Array Element` null)
    (`KismetArrayLibrary.Array_Add` (`self.Actors to Ignore`) (`GameplayStatics.GetPlayerPawn` 0))
    (if (== _array_element (`GameplayStatics.GetPlayerPawn` 0))
      _)))

(event `InputAxis|forward`
  (params (AxisValue :type "Float (single-precision)"))
  (bind _returnvalue (`GameplayStatics.GetPlayerPawn` 0))
  (`Pawn.AddMovementInput` _returnvalue (`self.GetActorForwardVector` _returnvalue) AxisValue false))

(event `InputAxis|Right`
  (params (AxisValue :type "Float (single-precision)"))
  (bind _returnvalue (`GameplayStatics.GetPlayerPawn` 0))
  (`Pawn.AddMovementInput` _returnvalue (`self.GetActorRightVector` _returnvalue) AxisValue false))

(event `InputAxis|lookup`
  (params (AxisValue :type "Float (single-precision)"))
  (`self.AddPitchInput` AxisValue))

(event `InputAxis|turn`
  (params (AxisValue :type "Float (single-precision)"))
  (`self.AddYawInput` AxisValue))

(event `InputAction|BodySwap`
  (params (Key :type "Key Structure"))
  (bind _actors_to_ignore (`self.Actors to Ignore`))
  (bind _camera (`/Game/Blueprints/BP_Player.Camera` (`self.Array Element`)))
  (bind _returnvalue (`SceneComponent.K2_GetComponentLocation` _camera))
  (:`Pressed`
    (bind _outactors (`GameplayStatics.GetAllActorsOfClass` "/Game/Blueprints/BP_Player.BP_Player_C"))
    (for _array_element _outactors
      (bind _output_get (set `self.Array Element` _array_element))
      (if (== _output_get (`GameplayStatics.GetPlayerPawn` 0))
        (`KismetSystemLibrary.PrintString` "Hello")
        (bind _outhit (`KismetSystemLibrary.LineTraceSingle` _returnvalue (+ _returnvalue (* (`SceneComponent.GetForwardVector` _camera) 10000.0)) "TraceTypeQuery1" false (`self.Actors to Ignore`) "ForDuration"))
        (bind (_bblockinghit _binitialoverlap _time _distance _location _impactpoint _normal _impactnormal _physmat _hitactor) (`GameplayStatics.BreakHitResult` _outhit))
        (if (`KismetStringLibrary.Contains` (`KismetSystemLibrary.GetDisplayName` _hitactor) "BP_Player")
          (message `/Game/Blueprints/PlayerScripts.Posses` _hitactor)
          (`KismetArrayLibrary.Array_Clear` _actors_to_ignore)
          (`KismetArrayLibrary.Array_Add` _actors_to_ignore (`GameplayStatics.GetPlayerPawn` 0)))))))

(event `Key|P`
  (params (Key :type "Key Structure"))
  (:`Pressed`
    (bind _returnvalue (`GameplayStatics.GetCurrentLevelName` true))
    (`GameplayStatics.OpenLevel` (`KismetStringLibrary.Conv_StringToName` _returnvalue))))

(event `Key|Escape`
  (params (Key :type "Key Structure"))
  (:`Pressed`
    (`KismetSystemLibrary.QuitGame` null "Quit")))

(event `InputAction|Interact`
  (params (Key :type "Key Structure"))
  (bind _camera (`/Game/Blueprints/BP_Player.Camera` (`self.Array Element`)))
  (bind _returnvalue (`SceneComponent.K2_GetComponentLocation` _camera))
  (:`Pressed`
    (bind _outactors (`GameplayStatics.GetAllActorsOfClass` "/Game/Blueprints/BP_Player.BP_Player_C"))
    (for _array_element _outactors
      (bind _output_get (set `self.Array Element` _array_element))
      (if (== _output_get (`GameplayStatics.GetPlayerPawn` 0))
        (bind (_outhit _returnvalue_2) (`KismetSystemLibrary.LineTraceSingle` _returnvalue (+ _returnvalue (* (`SceneComponent.GetForwardVector` _camera) 500.0)) "TraceTypeQuery1" false (`self.Actors to Ignore`) "ForDuration"))
        (if _returnvalue_2
          (`|ExecutionSequence`
            (:`then_0`
              (bind (_bblockinghit _binitialoverlap _time _distance _location _impactpoint _normal _impactnormal _physmat _hitactor _hitcomponent) (`GameplayStatics.BreakHitResult` _outhit))
              (message `/Game/Blueprints/Interactable.CanInteract` _hitactor))
            (:`then_1`
              (`PhysicsHandleComponent.GrabComponentAtLocationWithRotation` :`self` (`/Game/Blueprints/BP_Player.PhysicsHandle` (`self.Array Element`)) :`Component` _hitcomponent :`Location` (`SceneComponent.K2_GetComponentLocation` _hitcomponent))
              (set `self.IsGrabbingObject` true)))))))
  (:`Released`
    (if (`self.IsGrabbingObject`)
      (`PhysicsHandleComponent.ReleaseComponent` (`/Game/Blueprints/BP_Player.PhysicsHandle` (`self.Array Element`))))))

(event `self.ReceiveTick`
  (params (DeltaSeconds :type "Float (single-precision)"))
  (bind _array_element (`self.Array Element`))
  (if (`self.IsGrabbingObject`)
    (`PhysicsHandleComponent.SetTargetLocation` (`/Game/Blueprints/BP_Player.PhysicsHandle` _array_element) (`SceneComponent.K2_GetComponentLocation` (`/Game/Blueprints/BP_Player.GrabPoint` _array_element)))))

(fn `UserConstructionScript`)